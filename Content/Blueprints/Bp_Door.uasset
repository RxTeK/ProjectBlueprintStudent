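; Double door Blueprint that swings two door meshes open and closed when interacted with.
; The Interact event does nothing while the Key flag is true; otherwise a FlipFlop alternates between playing and reversing a Timeline.
; The Timeline's Rotation track, scaled by a separate angle variable for each door, drives the relative yaw of Door1 and Door2.
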(event `/Game/Blueprints/BPI_interact.Interact`
  (if (not (`self.Key ?`))
    (`/Engine/EditorBlueprintResources/StandardMacros.FlipFlop`
      (:`A`
        (bind (_direction _rotation) (`Timeline|Timeline` :!label _label)
          (:`Update`
            (`SceneComponent.K2_SetRelativeRotation` (`self.Door1`) (`KismetMathLibrary.MakeRotator` 0.0 0.0 (* _rotation (`self.AngleRotation1`))) false false)
            (`SceneComponent.K2_SetRelativeRotation` (`self.Door2`) (`KismetMathLibrary.MakeRotator` 0.0 0.0 (* _rotation (`self.AngleRotation2`))) false false))))
      (:`B`
        (goto _label :!via `Reverse`)))))

(fn `UserConstructionScript`)