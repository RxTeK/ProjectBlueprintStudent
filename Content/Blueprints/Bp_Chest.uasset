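; Chest Blueprint that opens its lid on interaction once a key value reaches exactly two.
; The Interact event checks the 2key variable, then plays the Open timeline, whose OpenChest track scales RotationOpen to rotate the cover mesh around roll.
; Tick prints the current key value to the screen every frame.
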(event `self.ReceiveTick`
  (params (DeltaSeconds :type "Float (single-precision)"))
  (`KismetSystemLibrary.PrintString` (`KismetStringLibrary.Conv_IntToString` (`self.2key?`)) true true (struct :`G` 0.66 :`B` 1.0 :`A` 1.0) 0.0))

(event `/Game/Blueprints/BPI_interact.Interact`
  (if (== (`self.2key?`) 2)
    (bind (_direction _open_chest) (`Timeline|open`)
      (:`Update`
        (`SceneComponent.K2_SetRelativeRotation` (`self.Chest_cover6_StaticMeshComponent0`) (`KismetMathLibrary.MakeRotator` (* _open_chest (`self.Rotation Open`))) false false)))))

(fn `UserConstructionScript`)